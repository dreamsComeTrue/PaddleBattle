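; Spawner actor for the Pong game that adds collide walls inside its box as play progresses.
; Every few paddle hits, set by the spawn rate, it spawns a wall up to a maximum count.
; Random locations snap to a grid and are tested, over limited tries, against cells used by walls and the power-up spawner.
; Game restart and next-round events from the game state destroy all spawned walls.
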(event Custom|GameRestartedEvent
  (CallFunction|RestartSpawner))

(event Custom|NextRoundEvent
  (CallFunction|RestartSpawner))

(event Custom|PointScoredEvent
  (params (Paddle :type BP%20Pong%20Paddle%20Object%20Reference) (HitCounter :type Integer))
  (if (== (Math|Integer|%(Integer) HitCounter (Variables|Default|GetCollideWallSpawnRate)) 0)
    (CallFunction|SpawnCollideWall)))

(event EventBeginPlay
  (bind _asbp_pong_game_state (Utilities|Casting|CastToBP_PongGameState (Game|GetGameState)))
  (EventDispatchers|BindEventtoOnGameRestarted _asbp_pong_game_state (delegate Custom|GameRestartedEvent))
  (EventDispatchers|BindEventtoOnNextRound _asbp_pong_game_state (delegate Custom|NextRoundEvent))
  (EventDispatchers|BindEventtoPaddleHit (Variables|Default|GetPongPlayer) (delegate Custom|PointScoredEvent)))

(fn ConstructionScript)

(fn RestartSpawner
  (bind _collidewalls (Variables|Default|GetCollideWalls))
  (bind _arrayelement (Utilities|Array|ReverseforEachLoop _collidewalls)
    (:LoopBody
      (Utilities|IsValid _arrayelement
        (:Is%20Valid
          (Actor|DestroyActor _arrayelement))))
    (:Completed
      (Utilities|Array|Clear _collidewalls))))

(fn SpawnCollideWall
  (if (< (Utilities|Array|Length (Variables|Default|GetCollideWalls)) (Variables|Default|GetMaxItemsToSpawn))
    (bind _location (CallFunction|CalculateCollideWallLocation))
    (bind _returnvalue (Game|SpawnActorfromClass "/Game/Blueprints/GamePlay/Objects/CollideWall/BP_CollideWall.BP_CollideWall_C" (Math|Transform|MakeTransform (Math|Vector|MakeVector (Math|Conversions|ToFloat(Integer) (.x _location)) (Math|Conversions|ToFloat(Integer) (.y _location)) 0.0) "0, 0, 0" "1,1,1") "AdjustIfPossibleButDontSpawnIfColliding" self 0))
    (Utilities|IsValid _returnvalue
      (:Is%20Valid
        (Utilities|Array|Add (Variables|Default|GetCollideWalls) _returnvalue)
        (Variables|/Game/Blueprints/GamePlay/Objects/CollideWall/BP_CollideWall.BP_CollideWall_C|SetGridLocation _returnvalue (Utilities|Struct|MakeIntVector (.x _location) (.y _location) 0))))))

(fn CalculateCollideWallLocation
  (bind _box (Variables|Default|GetBox))
  (bind _gridstep (Variables|Default|GetGridStep))
  (bind _gridstep_2 (Variables|Default|GetGridStep))
  (bind (_origin _boxextent) (Collision|GetComponentBounds _box))
  (bind _returnvalue (Math|Conversions|ToFloat(Integer) _gridstep))
  (bind _returnvalue_2 (Math|Conversions|ToFloat(Integer) _gridstep_2))
  (bind _returnvalue_3 (- (.x _origin) (.x _boxextent)))
  (bind _returnvalue_4 (- (.y _origin) (.y _boxextent)))
  (bind _returnvalue_5 (+ (.y _origin) (.y _boxextent)))
  (bind _returnvalue_6 (+ (.x _origin) (.x _boxextent)))
  (bind _returnvalue_7 (Math|Random|RandomFloatinRange _returnvalue_3 _returnvalue_6))
  (bind _returnvalue_8 (Math|Random|RandomFloatinRange _returnvalue_4 _returnvalue_5))
  (bind _returnvalue_9 (/ _returnvalue_8 _returnvalue))
  (bind _returnvalue_10 (/ _returnvalue_7 _returnvalue_2))
  (bind _returnvalue_11 (Math|Float|Truncate _returnvalue_9))
  (bind _returnvalue_12 (Math|Float|Truncate _returnvalue_10))
  (bind _returnvalue_13 (* _returnvalue_11 _gridstep))
  (bind _returnvalue_14 (* _returnvalue_12 _gridstep_2))
  (bind _locations (CallFunction|GetCollideWallsOccupiedLocations))
  (bind _output_get (LocalVariables|SetOccupiedLocations _locations))
  (bind _locations_2 (Default|GetPowerUpsOccupiedLocations (Variables|Default|GetPowerUpSpawner)))
  (Utilities|Array|AppendArray _output_get _locations_2)
  (Utilities|FlowControl|ForLoopwithBreak 0 (LocalVariables|GetNumberOfTries)
    (:LoopBody
      (if (not (Utilities|Array|ContainsItem (LocalVariables|GetOccupiedLocations) (Utilities|Struct|MakeIntVector _returnvalue_14 _returnvalue_13 0)))
        (return (Utilities|Struct|MakeIntVector _returnvalue_14 _returnvalue_13 0))))))

(fn GetCollideWallsOccupiedLocations
  (for _array_element (Variables|Default|GetCollideWalls)
    (Utilities|IsValid _array_element
      (:Is%20Valid
        (Utilities|Array|AddUnique (LocalVariables|GetCollideWallsLocations) (Variables|/Game/Blueprints/GamePlay/Objects/CollideWall/BP_CollideWall.BP_CollideWall_C|GetGridLocation _array_element)))))
  (return (LocalVariables|GetCollideWallsLocations)))