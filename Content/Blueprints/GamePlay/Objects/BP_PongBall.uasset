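; Pong ball that bounces off paddles and board walls and reports hits on score walls, reacting to game state events for rounds, restarts and game over.
; It sets physics velocity from a tracked velocity converted through the Anchor's transform.
; Paddle bounces blend hit offset, paddle velocity and randomness, with periodic speed-ups by turn count.
; Single mode scores paddle hits and ends on a score wall, while Classic and Hot Seat award points there.
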(event Custom|GameOverEvent
  ;[1 1 1] Register events handling
  (CallFunction|OnGameOver))

(event Custom|GameRestartEvent
  ;[1 1 1] Register events handling
  (CallFunction|OnGameRestarted))

(event Custom|PointScoredEvent
  (params (PlayerIndex :type Integer))
  ;[1 1 1] Register events handling
  (CallFunction|OnPointScored))

(event Custom|NextRoundEvent
  ;[1 1 1] Register events handling
  (CallFunction|OnNextRound))

(event EventBeginPlay
  (Utilities|FlowControl|Sequence
    (:then_0
      ;[1 1 1] Save Ball's initial location
      (Variables|Default|SetInitialLocation (Variables|/Script/Engine.SceneComponent|GetRelativeLocation (Variables|Default|GetBallMesh))))
    (:then_1
      ;[1 1 1] Register events handling
      (bind _asbp_pong_game_state (Utilities|Casting|CastToBP_PongGameState (Game|GetGameState)))
      (EventDispatchers|BindEventtoOnGameOver _asbp_pong_game_state (delegate Custom|GameOverEvent))
      (EventDispatchers|BindEventtoOnGameRestarted _asbp_pong_game_state (delegate Custom|GameRestartEvent))
      (EventDispatchers|BindEventtoOnPointScored _asbp_pong_game_state (delegate Custom|PointScoredEvent))
      (EventDispatchers|BindEventtoOnNextRound _asbp_pong_game_state (delegate Custom|NextRoundEvent)))
    (:then_2
      (Rendering|SetVisibility (Variables|Default|GetBallMesh) false true))))

(event Collision|EventActorBeginOverlap
  (params (OtherActor :type Actor%20Object%20Reference))
  ;[1 1 1] Ball overlapping with ScoreWall
  (bind _asbp_pong_score_wall (Utilities|Casting|CastToBP_PongScoreWall OtherActor))
  (CallFunction|CollidewithScoreWall (Variables|/Game/Blueprints/GamePlay/Level/BP_PongScoreWall.BP_PongScoreWall_C|GetPlayerIndex _asbp_pong_score_wall)))

(event Collision|EventHit
  (params (MyComp :type Primitive%20Component%20Object%20Reference) (Other :type Actor%20Object%20Reference) (OtherComp :type Primitive%20Component%20Object%20Reference) (bSelfMoved :type Boolean) (HitLocation :type Vector :default "0, 0, 0") (HitNormal :type Vector :default "0, 0, 0") (NormalImpulse :type Vector :default "0, 0, 0") (Hit :type Hit%20Result%20Structure%20%28by%20ref%29))
  ;[1 1 1] Ball hitting Paddle or BoardWall
  (if (!= Other (Variables|Default|GetLastHitObject))
    (bind _output_get (Variables|Default|SetLastHitObject Other))
    (bind _asbp_pong_paddle (Utilities|Casting|CastToBP_PongPaddle _output_get)
      (:then
        (CallFunction|CollidewithPaddle _asbp_pong_paddle HitLocation))
      (:CastFailed
        (Utilities|Casting|CastToBP_PongBoardWall Other)
        (CallFunction|CollidewithBoardWall)))))

(fn ConstructionScript)

(fn StartMoving
  (bind _ballmesh (Variables|Default|GetBallMesh))
  (Variables|Default|SetLastHitObject 0)
  (Physics|SetSimulatePhysics _ballmesh true)
  (Collision|SetCollisionEnabled _ballmesh "QueryAndPhysics")
  (Rendering|SetVisibility _ballmesh true true)
  (Variables|Default|SetCurrentSpeed (Math|Vector|MakeVector (Math|Float|Absolute(Float) (Variables|Default|GetInitialVelocity)) 0.0 0.0))
  (if (Variables|Default|GetFaceRight)
    _
    (else
      (Variables|Default|SetCurrentSpeed (* (Variables|Default|GetCurrentSpeed) -1.0))))
  (bind _outvector (CallFunction|LocaltoWorld (Variables|Default|GetCurrentSpeed)))
  (Physics|SetPhysicsLinearVelocity (Variables|Default|GetBallMesh) _outvector false "None")
  (Variables|Default|SetFaceRight (not (Variables|Default|GetFaceRight)))
  (bind _speed (CallFunction|GetBallSpeed))
  (Default|CallBallSpeedUpdated _speed))

(fn StopMoving
  (bind _ballmesh (Variables|Default|GetBallMesh))
  (Physics|SetPhysicsLinearVelocity _ballmesh "0, 0, 0" false "None")
  (Rendering|SetVisibility _ballmesh false true)
  (Physics|SetSimulatePhysics _ballmesh false)
  (Collision|SetCollisionEnabled _ballmesh "NoCollision")
  (Transformation|SetRelativeLocation _ballmesh (Variables|Default|GetInitialLocation) false true))

(fn LocaltoWorld
  (params (Vector :type Vector))
  (return (Math|Transform|InverseTransformDirection (Transformation|GetWorldTransform (Variables|Default|GetAnchor)) Vector)))

(fn WorldtoLocal
  (params (Vector :type Vector))
  (return (Math|Transform|TransformDirection (Transformation|GetWorldTransform (Variables|Default|GetAnchor)) Vector)))

(fn CollidewithPaddle
  (params (Paddle :type BP%20Pong%20Paddle%20Object%20Reference) (HitLocation :type Vector))
  (Utilities|SwitchonGameType
    (:Single
      ;[1 1 1] Score point everytime a (either) paddle is hit
      (bind _asbp_pong_game_state (Utilities|Casting|CastToBP_PongGameState (Game|GetGameState)))
      (Default|ScorePoint _asbp_pong_game_state))
    (:Classic
      _)
    (:Hot%20Seat
      _))
  (CallFunction|PaddleBallBounce Paddle (Math|Transform|InverseTransformLocation (Transformation|GetActorTransform Paddle) HitLocation))
  (CallFunction|IncreaseBallSpeed)
  (bind _speed (CallFunction|GetBallSpeed))
  (Default|CallBallSpeedUpdated _speed))

(fn CollidewithBoardWall
  (bind _output_get (Variables|Default|SetCurrentSpeed (Math|Vector|MakeVector (.x (Variables|Default|GetCurrentSpeed)) (* (.y (Variables|Default|GetCurrentSpeed)) -1.0) (.z (Variables|Default|GetCurrentSpeed)))))
  (bind _outvector (CallFunction|LocaltoWorld _output_get))
  (Physics|SetPhysicsLinearVelocity (Variables|Default|GetBallMesh) _outvector false "None")
  (bind _speed (CallFunction|GetBallSpeed))
  (Default|CallBallSpeedUpdated _speed))

(fn CollidewithScoreWall
  (params (PlayerIndex :type Integer))
  (bind _asbp_pong_game_state (Utilities|Casting|CastToBP_PongGameState (Game|GetGameState)))
  (Utilities|SwitchonGameType
    (:Single
      (Default|PongGameOver _asbp_pong_game_state))
    (:Classic
      (Default|ScorePoint _asbp_pong_game_state PlayerIndex :!label _label)
      (CallFunction|StopMoving))
    (:Hot%20Seat
      (goto _label))))

(fn PaddleBallBounce
  (params (Paddle :type BP%20Pong%20Paddle%20Object%20Reference) (HitLocation :type Vector))
  (bind _paddlemesh (Variables|/Game/Blueprints/GamePlay/Player/BP_PongPaddle.BP_PongPaddle_C|GetPaddleMesh Paddle))
  (bind (_min _max) (Components|StaticMesh|GetLocalBounds _paddlemesh))
  (bind _returnvalue (Physics|GetPhysicsLinearVelocity (Variables|/Game/Blueprints/GamePlay/Player/BP_PongPaddle.BP_PongPaddle_C|GetPaddleMesh Paddle) "None"))
  (bind _outvector (CallFunction|WorldtoLocal _returnvalue))
  (bind _output_get (Variables|Default|SetCurrentSpeed (Math|Vector|MakeVector (* (.x (Variables|Default|GetCurrentSpeed)) -1.0) (+ (/ (.y _outvector) 2.0) (* (Math|Float|MapRangeClamped (.y HitLocation) (.y _min) (.y _max) -128.0 128.0) (Math|Random|RandomFloatinRange 0.5 (Variables|Default|GetPaddleBounceRandomSpread)))) (.z (Variables|Default|GetCurrentSpeed)))))
  (bind _outvector_2 (CallFunction|LocaltoWorld _output_get))
  (Physics|SetPhysicsLinearVelocity (Variables|Default|GetBallMesh) _outvector_2 false "None"))

(fn IncreaseBallSpeed
  (bind _asbp_pong_game_state (Utilities|Casting|CastToBP_PongGameState (Game|GetGameState)))
  (bind _asbp_pong_game_mode (Utilities|Casting|CastToBP_PongGameMode (Game|GetGameMode)))
  (if (== (Math|Integer|%(Integer) (Variables|/Game/Blueprints/GamePlay/BP_PongGameState.BP_PongGameState_C|GetTurnsCounter _asbp_pong_game_state) (Variables|/Game/Blueprints/GamePlay/BP_PongGameMode.BP_PongGameMode_C|GetBallSpeedIncreaseTurns _asbp_pong_game_mode)) 0)
    (bind _output_get (Variables|Default|SetCurrentSpeed (+ (Variables|Default|GetCurrentSpeed) (* (Variables|Default|GetCurrentSpeed) (Variables|/Game/Blueprints/GamePlay/BP_PongGameMode.BP_PongGameMode_C|GetBallSpeedIncreaseAmount _asbp_pong_game_mode)))))
    (bind _outvector (CallFunction|LocaltoWorld _output_get))
    (Physics|SetPhysicsLinearVelocity (Variables|Default|GetBallMesh) _outvector false "None")))

(fn GetBallSpeed
  (return (Math|Vector|VectorLength (/ (Variables|Default|GetCurrentSpeed) 1e+02))))

(fn OnGameOver
  (CallFunction|StopMoving))

(fn OnGameRestarted
  (bind _ballmesh (Variables|Default|GetBallMesh))
  (Transformation|SetRelativeLocation _ballmesh (Variables|Default|GetInitialLocation) false true)
  (Physics|SetSimulatePhysics _ballmesh true)
  (Collision|SetCollisionEnabled _ballmesh "QueryAndPhysics")
  (Utilities|Time|SetTimerbyEvent (EventDispatchers|CreateEvent :!event StartMoving) 1.0))

(fn OnPointScored)

(fn OnNextRound
  (Utilities|Time|SetTimerbyEvent (EventDispatchers|CreateEvent :!event StartMoving) (Variables|Default|GetWaitTimeBetweenRounds)))