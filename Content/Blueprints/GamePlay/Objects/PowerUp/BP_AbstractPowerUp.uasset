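; BP_AbstractPowerUp is a base Blueprint for power-up objects created under a BP_PowerUpSpawner.
; GetPowerUpText and GetPowerUpColor are placeholders returning empty or default values, apparently for child Blueprints to override.
; IncreaseAge increments an Age counter.
; When destroyed, the power-up casts its owner to the spawner and removes itself from that spawner's PowerUps collection.
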(event EventDestroyed
  (bind _asbp_power_up_spawner (Utilities|Casting|CastToBP_PowerUpSpawner (Components|GetOwner)))
  (Utilities|Array|RemoveItem (Variables|/Game/Blueprints/GamePlay/Objects/PowerUp/BP_PowerUpSpawner.BP_PowerUpSpawner_C|GetPowerUps _asbp_power_up_spawner) self))

(fn ConstructionScript)

(fn GetPowerUpText
  (return ""))

(fn GetPowerUpColor
  (return ""))

(fn IncreaseAge
  (Math|Integer|IncrementInt (Variables|Default|GetAge)))