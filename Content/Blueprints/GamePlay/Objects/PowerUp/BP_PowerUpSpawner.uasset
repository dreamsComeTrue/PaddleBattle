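; Spawner actor that drops random power-ups inside a box area during a Pong match.
; Every SpawnRate-th hit reported by the player paddle ages the tracked power-ups, then spawns a random class at a random X/Y within the box.
; Once the tracked array reaches its cap, spawning requires destroying the first valid power-up past maximum age; destroyed entries stay in the array.
; Game restart and next-round events destroy all power-ups and clear the array.
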(event Custom|GameRestartedEvent
  (CallFunction|RestartSpawner))

(event Custom|NextRoundEvent
  (CallFunction|RestartSpawner))

(event Custom|PointScoredEvent
  (params (Paddle :type BP%20Pong%20Paddle%20Object%20Reference) (HitCounter :type Integer))
  (if (== (Math|Integer|%(Integer) HitCounter (Variables|Default|GetSpawnRate)) 0)
    (CallFunction|SpawnPowerUp)))

(event EventBeginPlay
  (bind _asbp_pong_game_state (Utilities|Casting|CastToBP_PongGameState (Game|GetGameState)))
  (EventDispatchers|BindEventtoOnGameRestarted _asbp_pong_game_state (delegate Custom|GameRestartedEvent))
  (EventDispatchers|BindEventtoOnNextRound _asbp_pong_game_state (delegate Custom|NextRoundEvent))
  (bind _asbp_pong_player (Utilities|Casting|CastToBP_PongPlayer (Game|Player|GetPlayerPawn 0)))
  (EventDispatchers|BindEventtoPaddleHit _asbp_pong_player (delegate Custom|PointScoredEvent)))

(fn ConstructionScript)

(fn RestartSpawner
  (bind _arrayelement (Utilities|Array|ReverseforEachLoop (Variables|Default|GetPowerUps))
    (:LoopBody
      (Utilities|IsValid _arrayelement
        (:Is%20Valid
          (Actor|DestroyActor _arrayelement))))
    (:Completed
      (Utilities|Array|Clear (Variables|Default|GetPowerUps)))))

(fn SpawnPowerUp
  (CallFunction|UpdatePowerUpsAge)
  (if (< (Utilities|Array|Length (Variables|Default|GetPowerUps)) (Variables|Default|GetMaxItemsToSpawn))
    (CallFunction|CreateRandomPowerUp)
    (else
      (bind _was_removed (CallFunction|RemoveOldestPowerUp))
      (if _was_removed
        (CallFunction|CreateRandomPowerUp)))))

(fn CreateRandomPowerUp
  (bind _box (Variables|Default|GetBox))
  (bind (_origin _boxextent) (Collision|GetComponentBounds _box))
  (bind _returnvalue (Game|SpawnActorfromClass (Utilities|Array|Get(acopy) (Variables|Default|GetPowerUpsClasses) (Math|Random|RandomIntegerinRange 0 (- (Utilities|Array|Length (Variables|Default|GetPowerUpsClasses)) 1))) (Math|Transform|MakeTransform (Math|Vector|MakeVector (Math|Random|RandomFloatinRange (- (.x _origin) (.x _boxextent)) (+ (.x _origin) (.x _boxextent))) (Math|Random|RandomFloatinRange (- (.y _origin) (.y _boxextent)) (+ (.y _origin) (.y _boxextent))) 0.0) "0, 0, 0" "1,1,1") "AlwaysSpawn" self 0))
  (Utilities|Array|Add (Variables|Default|GetPowerUps) _returnvalue))

(fn RemoveOldestPowerUp
  (bind _array_element (Utilities|Array|ForEachLoopwithBreak (Variables|Default|GetPowerUps) :!label _label)
    (:LoopBody
      (Utilities|IsValid _array_element
        (:Is%20Valid
          (if (>= (Variables|/Game/Blueprints/GamePlay/Objects/PowerUp/BP_AbstractPowerUp.BP_AbstractPowerUp_C|GetAge _array_element) (Variables|Default|GetMaxPowerUpAge))
            (Actor|DestroyActor _array_element)
            (LocalVariables|SetWasRemoved true)
            (goto _label Break)))))
    (:Completed
      (return (LocalVariables|GetWasRemoved)))))

(fn UpdatePowerUpsAge
  (for _array_element (Variables|Default|GetPowerUps)
    (Utilities|IsValid _array_element
      (:Is%20Valid
        (Default|IncreaseAge _array_element)))))