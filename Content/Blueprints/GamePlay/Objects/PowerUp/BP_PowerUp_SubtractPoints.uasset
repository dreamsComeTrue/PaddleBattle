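; Power-up that makes the paddle it is applied to lose a random number of points.
; On BeginPlay it rolls an amount between one and MaxRandomPoints and stores it as a negative value.
; ApplyPowerUpEffect passes that negative value to SubtractPoints on a valid paddle.
; Text and color overrides supply a red "Subtract Points!" label with the amount appended.
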(event EventBeginPlay
  (|CallParentFunction)
  (Variables|Default|SetPointsToSubtract (* (Math|Random|RandomIntegerinRange 1 (Variables|Default|GetMaxRandomPoints)) -1)))

(event Collision|EventActorBeginOverlap
  (params (OtherActor :type Actor%20Object%20Reference))
  (|CallParentFunction OtherActor) ; This node is disabled and will not be called.\nDrag off pins to build functionality.
)

(event EventTick
  (params (DeltaSeconds :type Float%20%28single-precision%29))
  (|CallParentFunction DeltaSeconds) ; This node is disabled and will not be called.\nDrag off pins to build functionality.
)

(event EventApplyPowerUpEffect
  (params (Ball :type BP%20Pong%20Ball%20Object%20Reference) (Paddle :type BP%20Pong%20Paddle%20Object%20Reference))
  (Utilities|IsValid Paddle
    (:Is%20Valid
      (Default|SubtractPoints Paddle (Variables|Default|GetPointsToSubtract)))))

(fn ConstructionScript
  (|CallParentFunction))

(fn GetPowerUpText
  (return (Utilities|Text|ToText(String) (Utilities|String|Append "Subtract Points! " (Utilities|String|ToString(Integer) (Variables|Default|GetPointsToSubtract))))))

(fn GetPowerUpColor
  (return (Utilities|Struct|MakeSlateColor "(R=1.000000,G=0.000000,B=0.000000,A=1.000000)")))