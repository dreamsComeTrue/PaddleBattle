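; World-space score display for Pong, using text render components under separate anchors for single and two-score layouts.
; Binds to the game state's restart and point-scored events to refresh the numbers, also updating anchor visibility on restart.
; A macro branches on the game mode's Pong type: Single shows only the left player's score, while Classic and Hot Seat show both.
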(event Custom|PointScored
  (params (PlayerIndex :type Integer))
  (CallFunction|UpdatePointsUI))

(event Custom|GameRestarted
  (CallFunction|SetUIVisbility)
  (CallFunction|UpdatePointsUI))

(event EventBeginPlay
  (bind _asbp_pong_game_state (Utilities|Casting|CastToBP_PongGameState (Game|GetGameState)))
  (EventDispatchers|BindEventtoOnGameRestarted _asbp_pong_game_state (delegate Custom|GameRestarted))
  (EventDispatchers|BindEventtoOnPointScored _asbp_pong_game_state (delegate Custom|PointScored)))

(fn ConstructionScript)

(fn SetUIVisbility
  (Utilities|SwitchonPongGameType
    (:Single
      (Rendering|SetVisibility (Variables|Default|GetClassicGameTypeAnchor) false true)
      (Rendering|SetVisibility (Variables|Default|GetSingleGameTypeAnchor) true true))
    (:Classic
      (Rendering|SetVisibility (Variables|Default|GetClassicGameTypeAnchor) true true :!label _label)
      (Rendering|SetVisibility (Variables|Default|GetSingleGameTypeAnchor) false true))
    (:Hot%20Seat
      (goto _label))))

(fn SetSingleGamePoints
  (params (Value :type Integer))
  (Rendering|Components|TextRender|SetText (Variables|Default|GetSingle_Points_TextRender) (Utilities|Text|ToText(Integer) Value)))

(fn SetClassicGamePoints
  (params (Player%20Left%20Score :type Integer) (Player%20Right%20Score :type Integer))
  (Rendering|Components|TextRender|SetText (Variables|Default|GetClassic_Left_Points_TextRender) (Utilities|Text|ToText(Integer) Player%20Left%20Score))
  (Rendering|Components|TextRender|SetText (Variables|Default|GetClassic_Right_Points_TextRender) (Utilities|Text|ToText(Integer) Player%20Right%20Score)))

(fn UpdatePointsUI
  (bind _asbp_pong_game_state (Utilities|Casting|CastToBP_PongGameState (Game|GetGameState)))
  (Utilities|SwitchonPongGameType
    (:Single
      (CallFunction|SetSingleGamePoints (Variables|/Game/Blueprints/GamePlay/BP_PongGameState.BP_PongGameState_C|GetPlayerLeft_Score _asbp_pong_game_state)))
    (:Classic
      (CallFunction|SetClassicGamePoints (Variables|/Game/Blueprints/GamePlay/BP_PongGameState.BP_PongGameState_C|GetPlayerLeft_Score _asbp_pong_game_state) (Variables|/Game/Blueprints/GamePlay/BP_PongGameState.BP_PongGameState_C|GetPlayerRight_Score _asbp_pong_game_state) :!label _label))
    (:Hot%20Seat
      (goto _label))))