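; Physics-driven Pong ball that bounces off paddles and board walls, reports scoring to BP_PongGameState, and alternates launch direction on each serve.
; Overlaps dispatch by actor type, with bounces flipping velocity in the Anchor's frame and paddles adding their lateral velocity.
; Single mode scores paddle hits and ends on a score wall; Classic scores at score walls and re-serves.
; Game state events hide and freeze the ball or relaunch it.
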(event Custom|GameOverEvent
  ;[1 1 1] Register GameOver handling
  (CallFunction|GameOver))

(event Custom|GameRestartEvent
  ;[1 1 1] Register GameOver handling
  (CallFunction|GameRestart))

(event EventBeginPlay
  (Utilities|FlowControl|Sequence
    (:then_0
      ;[1 1 1] Save Ball's initial location
      (Variables|Default|SetInitialLocation (Variables|/Script/Engine.SceneComponent|GetRelativeLocation (Variables|Default|GetStaticMesh))))
    (:then_1
      ;[1 1 1] Register GameOver handling
      (bind _asbp_pong_game_state (Utilities|Casting|CastToBP_PongGameState (Game|GetGameState)))
      (EventDispatchers|BindEventtoOnGameOver _asbp_pong_game_state (delegate Custom|GameOverEvent))
      (EventDispatchers|BindEventtoOnGameRestarted _asbp_pong_game_state (delegate Custom|GameRestartEvent)))))

(event Collision|EventActorBeginOverlap
  (params (OtherActor :type Actor%20Object%20Reference))
  ;[1 1 1] Ball overlapping with game objects
  (bind _asbp_pong_paddle (Utilities|Casting|CastToBP_PongPaddle OtherActor)
    (:then
      (CallFunction|CollidewithPaddle _asbp_pong_paddle))
    (:CastFailed
      (Utilities|Casting|CastToBP_PongBoardWall OtherActor
        (:then
          (CallFunction|CollidewithBoardWall))
        (:CastFailed
          (bind _asbp_pong_score_wall (Utilities|Casting|CastToBP_PongScoreWall OtherActor))
          (CallFunction|CollidewithScoreWall (Variables|/Game/Blueprints/GamePlay/Level/BP_PongScoreWall.BP_PongScoreWall_C|GetPlayerIndex _asbp_pong_score_wall)))))))

(fn ConstructionScript)

(fn StartMoving
  (LocalVariables|SetVelocity (Math|Vector|MakeVector 0.0 (Math|Float|Absolute(Float) (Variables|Default|GetInitialVelocity)) 0.0))
  (if (Variables|Default|GetFaceRight)
    _
    (else
      (bind _output_get (LocalVariables|SetVelocity (* (LocalVariables|GetVelocity) -1.0)))))
  (Physics|SetPhysicsLinearVelocity (Variables|Default|GetStaticMesh) _output_get false "None")
  (Variables|Default|SetFaceRight (not (Variables|Default|GetFaceRight))))

(fn LocaltoWorld
  (params (Vector :type Vector))
  (return (Math|Transform|InverseTransformDirection (Transformation|GetWorldTransform (Variables|Default|GetAnchor)) Vector)))

(fn WorldtoLocal
  (params (Vector :type Vector))
  (return (Math|Transform|TransformDirection (Transformation|GetWorldTransform (Variables|Default|GetAnchor)) Vector)))

(fn CollidewithPaddle
  (params (Paddle :type BP%20Pong%20Paddle%20Object%20Reference))
  (Utilities|SwitchonGameType
    (:Single
      ;[1 1 1] Score point everytime a (either) paddle is hit
      (bind _asbp_pong_game_state (Utilities|Casting|CastToBP_PongGameState (Game|GetGameState)))
      (Default|ScorePoint _asbp_pong_game_state))
    (:Classic
      _))
  (CallFunction|PaddleBallBounce Paddle))

(fn CollidewithBoardWall
  (bind _returnvalue (Physics|GetPhysicsLinearVelocity (Variables|Default|GetStaticMesh) "None"))
  (bind _outvector (CallFunction|WorldtoLocal _returnvalue))
  (bind _outvector_2 (CallFunction|LocaltoWorld (Math|Vector|MakeVector (* (.x _outvector) -1.0) (.y _outvector) (.z _outvector))))
  (Physics|SetPhysicsLinearVelocity (Variables|Default|GetStaticMesh) _outvector_2 false "None"))

(fn CollidewithScoreWall
  (params (PlayerIndex :type Integer))
  (bind _asbp_pong_game_state (Utilities|Casting|CastToBP_PongGameState (Game|GetGameState)))
  (Utilities|SwitchonGameType
    (:Single
      (Default|PongGameOver _asbp_pong_game_state))
    (:Classic
      (Default|ScorePoint _asbp_pong_game_state PlayerIndex)
      (Transformation|SetRelativeLocation (Variables|Default|GetStaticMesh) (Variables|Default|GetInitialLocation) false true)
      (CallFunction|StartMoving))))

(fn PaddleBallBounce
  (params (Paddle :type BP%20Pong%20Paddle%20Object%20Reference))
  (bind _returnvalue (Physics|GetPhysicsLinearVelocity (Variables|Default|GetStaticMesh) "None"))
  (bind _outvector (CallFunction|WorldtoLocal _returnvalue))
  (bind _returnvalue_2 (Physics|GetPhysicsLinearVelocity (Variables|/Game/Blueprints/GamePlay/Player/BP_PongPaddle.BP_PongPaddle_C|GetStaticMesh Paddle) "None"))
  (bind _outvector_2 (CallFunction|WorldtoLocal _returnvalue_2))
  (bind _outvector_3 (CallFunction|LocaltoWorld (Math|Vector|MakeVector (+ (.x _outvector) (.x _outvector_2)) (* (.y _outvector) -1.0) (.z _outvector))))
  (Physics|SetPhysicsLinearVelocity (Variables|Default|GetStaticMesh) _outvector_3 false "None"))

(fn GameOver
  (Physics|SetPhysicsLinearVelocity (Variables|Default|GetStaticMesh) "0, 0, 0" false "None")
  (Rendering|SetVisibility (Variables|Default|GetStaticMesh) false true)
  (Physics|SetSimulatePhysics (Variables|Default|GetStaticMesh) false)
  (Collision|SetCollisionEnabled (Variables|Default|GetStaticMesh) "NoCollision"))

(fn GameRestart
  (Transformation|SetRelativeLocation (Variables|Default|GetStaticMesh) (Variables|Default|GetInitialLocation) false true)
  (Physics|SetSimulatePhysics (Variables|Default|GetStaticMesh) true)
  (Collision|SetCollisionEnabled (Variables|Default|GetStaticMesh) "QueryAndPhysics")
  (Rendering|SetVisibility (Variables|Default|GetStaticMesh) true true)
  (CallFunction|StartMoving))