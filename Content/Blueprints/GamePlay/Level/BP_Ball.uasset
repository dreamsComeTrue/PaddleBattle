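; Pong-style ball that bounces off board walls and paddles and reports points when it overlaps a score wall.
; StartMove serves it along the Y axis at an initial speed, alternating direction after each serve.
; Overlaps set physics velocity directly through local/world conversion helpers: walls flip X, while paddles flip Y and add their own X/Y velocity.
; Score walls pass their player index to ScorePoint, then the ball teleports to its start and serves again.
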(event EventBeginPlay
  (Variables|Default|SetInitialLocation (Variables|/Script/Engine.SceneComponent|GetRelativeLocation (Variables|Default|GetStaticMesh)))
  (CallFunction|StartMove))

(event Collision|EventActorBeginOverlap
  (params (OtherActor :type Actor%20Object%20Reference))
  (bind _staticmesh (Variables|Default|GetStaticMesh))
  (bind _staticmesh_2 (Variables|Default|GetStaticMesh))
  (Utilities|Casting|CastToBP_BoardWall OtherActor
    (:then
      (bind _returnvalue (Physics|GetPhysicsLinearVelocity _staticmesh "None"))
      (Physics|SetPhysicsLinearVelocity _staticmesh (Utilities|LocaltoWorld (Math|Vector|MakeVector (* (.X (Math|Vector|BreakVector (Utilities|WorldtoLocal _returnvalue))) -1.0) (.Y (Math|Vector|BreakVector (Utilities|WorldtoLocal _returnvalue))) (.Z (Math|Vector|BreakVector (Utilities|WorldtoLocal _returnvalue))))) false "None"))
    (:CastFailed
      (bind _asbp_score_wall (Utilities|Casting|CastToBP_ScoreWall OtherActor)
        (:then
          (Default|CallScorePoint (Variables|/Script/PaddleBattle.ScoreWall|GetPlayerIndex _asbp_score_wall))
          (Transformation|SetRelativeLocation (Variables|Default|GetStaticMesh) (Variables|Default|GetInitialLocation) false true)
          (CallFunction|StartMove))
        (:CastFailed
          (bind _asbp_paddle (Utilities|Casting|CastToBP_Paddle OtherActor))
          (bind _returnvalue_2 (Physics|GetPhysicsLinearVelocity _staticmesh_2 "None"))
          (bind _returnvalue_3 (Physics|GetPhysicsLinearVelocity (Variables|/Script/PaddleBattle.Paddle|GetPaddleMesh _asbp_paddle) "None"))
          (Physics|SetPhysicsLinearVelocity _staticmesh_2 (Utilities|LocaltoWorld (Math|Vector|MakeVector (+ (.x (Utilities|WorldtoLocal _returnvalue_3)) (.x (Math|Vector|MakeVector (.X (Math|Vector|BreakVector (Utilities|WorldtoLocal _returnvalue_2))) (* (.Y (Math|Vector|BreakVector (Utilities|WorldtoLocal _returnvalue_2))) -1.0) (.Z (Math|Vector|BreakVector (Utilities|WorldtoLocal _returnvalue_2)))))) (+ (.y (Utilities|WorldtoLocal _returnvalue_3)) (.y (Math|Vector|MakeVector (.X (Math|Vector|BreakVector (Utilities|WorldtoLocal _returnvalue_2))) (* (.Y (Math|Vector|BreakVector (Utilities|WorldtoLocal _returnvalue_2))) -1.0) (.Z (Math|Vector|BreakVector (Utilities|WorldtoLocal _returnvalue_2)))))) (.z (Math|Vector|MakeVector (.X (Math|Vector|BreakVector (Utilities|WorldtoLocal _returnvalue_2))) (* (.Y (Math|Vector|BreakVector (Utilities|WorldtoLocal _returnvalue_2))) -1.0) (.Z (Math|Vector|BreakVector (Utilities|WorldtoLocal _returnvalue_2))))))) false "None"))))))

(fn ConstructionScript)

(fn StartMove
  (if (Variables|Default|GetFaceRight)
    (Physics|SetPhysicsLinearVelocity (Variables|Default|GetStaticMesh) (Math|Vector|MakeVector 0.0 (Variables|Default|GetInitialVelocity) 0.0) false "None")
    (else
      (Physics|SetPhysicsLinearVelocity (Variables|Default|GetStaticMesh) (Math|Vector|MakeVector 0.0 (* (Variables|Default|GetInitialVelocity) -1.0) 0.0) false "None")))
  (Variables|Default|SetFaceRight (not (Variables|Default|GetFaceRight))))