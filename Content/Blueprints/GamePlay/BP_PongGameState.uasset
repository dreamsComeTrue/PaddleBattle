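; Game state Blueprint for a Pong game that tracks left and right player scores and a turn counter.
; Scoring a point increments the scorer and turn count, fires a point-scored dispatcher, then checks the Classic win limit read from BP_PongGameMode.
; Game over fires a dispatcher, shows the WB_GameOver widget and switches to UI-only input with a cursor.
; Restart zeroes all counters and broadcasts the reset.
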(event Custom|ScorePoint
  (params (PlayerIndex :type Integer))
  (if (== PlayerIndex 0)
    (Math|Integer|IncrementInt (Variables|Default|GetPlayerLeft_Score)
      (:%20%20
        _))
    (else
      (Math|Integer|IncrementInt (Variables|Default|GetPlayerRight_Score)
        (:%20%20
          _))))
  (CallFunction|IncreaseTurnsCounter)
  (Default|CallOnPointScored PlayerIndex)
  (CallFunction|CheckClassicGameTypeWinConditions))

(event Custom|PongGameOver
  (bind _returnvalue (Game|GetPlayerController 0))
  (Default|CallOnGameOver)
  (bind _returnvalue_2 (UserInterface|CreateWidget "/Game/Blueprints/UI/WB_GameOver.WB_GameOver_C" _returnvalue))
  (UserInterface|Viewport|AddtoPlayerScreen _returnvalue_2)
  (Input|SetInputModeUIOnly _returnvalue 0 "DoNotLock")
  (Variables|/Script/Engine.PlayerController|SetbShowMouseCursor _returnvalue true))

(event Custom|RestartPongGame
  (Variables|Default|SetPlayerLeft_Score 0)
  (Variables|Default|SetPlayerRight_Score 0)
  (Variables|Default|SetTurnsCounter 0)
  (Default|CallOnGameRestarted))

(fn ConstructionScript)

(fn CheckClassicGameTypeWinConditions
  (bind _asbp_pong_game_mode (Utilities|Casting|CastToBP_PongGameMode (Game|GetGameMode)))
  (switch Utilities|FlowControl|Switch|SwitchonEPongGameType (Variables|/Game/Blueprints/GamePlay/BP_PongGameMode.BP_PongGameMode_C|GetPongGameType _asbp_pong_game_mode)
    (:NewEnumerator1
      (if (or (>= (Variables|Default|GetPlayerLeft_Score) (Variables|/Game/Blueprints/GamePlay/BP_PongGameMode.BP_PongGameMode_C|GetClassicModePointsLimit _asbp_pong_game_mode)) (>= (Variables|Default|GetPlayerRight_Score) (Variables|/Game/Blueprints/GamePlay/BP_PongGameMode.BP_PongGameMode_C|GetClassicModePointsLimit _asbp_pong_game_mode)))
        (CallFunction|PongGameOver)))))

(fn IncreaseTurnsCounter
  (Math|Integer|IncrementInt (Variables|Default|GetTurnsCounter)))