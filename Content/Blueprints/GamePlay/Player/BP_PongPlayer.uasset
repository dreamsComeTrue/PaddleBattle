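; Player Blueprint for Pong that spawns and controls both the left and right paddles.
; On BeginPlay it spawns two BP_PongPaddle actors mirrored on Y by PaddlesDistance, using the PaddleAnchor's relative X and Z, and gives them a white material.
; Separate up and down input axes for each paddle call its movement functions, passing a shared MovementSpeed and the relative location of the TopBounds or BottomBounds component as the limit.
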(event EventBeginPlay
  (bind _paddleanchor (Variables|Default|GetPaddleAnchor))
  (bind _paddleanchor_2 (Variables|Default|GetPaddleAnchor))
  (bind _relativelocation (Variables|/Script/Engine.SceneComponent|GetRelativeLocation _paddleanchor))
  (bind _relativelocation_2 (Variables|/Script/Engine.SceneComponent|GetRelativeLocation _paddleanchor_2))
  ;[1 1 1] Spawn Left Paddle
  (bind _returnvalue (Game|SpawnActorfromClass "/Game/Blueprints/GamePlay/Player/BP_PongPaddle.BP_PongPaddle_C" (Math|Transform|MakeTransform (Math|Vector|MakeVector (.x _relativelocation_2) (* (Variables|Default|GetPaddlesDistance) -1.0) (.z _relativelocation_2)) "0, 0, 0" "1,1,1") "Undefined" 0 0))
  (bind _output_get (Variables|Default|SetLeftPaddle _returnvalue))
  (Rendering|Material|SetMaterial (Variables|/Game/Blueprints/GamePlay/Player/BP_PongPaddle.BP_PongPaddle_C|GetStaticMesh _output_get) 0 "/Game/Materials/MT_PongWhite.MT_PongWhite")
  ;[1 1 1] Spawn Right Paddle
  (bind _returnvalue_2 (Game|SpawnActorfromClass "/Game/Blueprints/GamePlay/Player/BP_PongPaddle.BP_PongPaddle_C" (Math|Transform|MakeTransform (Math|Vector|MakeVector (.x _relativelocation) (Variables|Default|GetPaddlesDistance) (.z _relativelocation)) "0, 0, 0" "1,1,1") "Undefined" 0 0))
  (bind _output_get_2 (Variables|Default|SetRightPaddle _returnvalue_2))
  (Rendering|Material|SetMaterial (Variables|/Game/Blueprints/GamePlay/Player/BP_PongPaddle.BP_PongPaddle_C|GetStaticMesh _output_get_2) 0 "/Game/Materials/MT_PongWhite.MT_PongWhite"))

(event Input|AxisEvents|InputAxisLeftPaddleDown
  (params (AxisValue :type Float%20%28single-precision%29))
  (bind _leftpaddle (Variables|Default|GetLeftPaddle))
  ;[1 1 1] Left Paddle Down
  (Utilities|IsValid _leftpaddle
    (:Is%20Valid
      (Default|MovePaddleDown _leftpaddle (Variables|Default|GetMovementSpeed) AxisValue (Variables|/Script/Engine.SceneComponent|GetRelativeLocation (Variables|Default|GetBottomBounds))))))

(event Input|AxisEvents|InputAxisLeftPaddleUp
  (params (AxisValue :type Float%20%28single-precision%29))
  (bind _leftpaddle (Variables|Default|GetLeftPaddle))
  ;[1 1 1] Left Paddle Up
  (Utilities|IsValid _leftpaddle
    (:Is%20Valid
      (Default|MovePaddleUp _leftpaddle (Variables|Default|GetMovementSpeed) AxisValue (Variables|/Script/Engine.SceneComponent|GetRelativeLocation (Variables|Default|GetTopBounds))))))

(event Input|AxisEvents|InputAxisRightPaddleUp
  (params (AxisValue :type Float%20%28single-precision%29))
  (bind _rightpaddle (Variables|Default|GetRightPaddle))
  ;[1 1 1] Right Paddle Up
  (Utilities|IsValid _rightpaddle
    (:Is%20Valid
      (Default|MovePaddleUp _rightpaddle (Variables|Default|GetMovementSpeed) AxisValue (Variables|/Script/Engine.SceneComponent|GetRelativeLocation (Variables|Default|GetTopBounds))))))

(event Input|AxisEvents|InputAxisRightPaddleDown
  (params (AxisValue :type Float%20%28single-precision%29))
  (bind _rightpaddle (Variables|Default|GetRightPaddle))
  ;[1 1 1] Right Paddle Down
  (Utilities|IsValid _rightpaddle
    (:Is%20Valid
      (Default|MovePaddleDown _rightpaddle (Variables|Default|GetMovementSpeed) AxisValue (Variables|/Script/Engine.SceneComponent|GetRelativeLocation (Variables|Default|GetBottomBounds))))))

(fn ConstructionScript)