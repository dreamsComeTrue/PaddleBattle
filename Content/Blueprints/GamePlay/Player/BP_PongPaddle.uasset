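; BP_PongPaddle is the player paddle actor for Pong, with movement, resizing and scoring functions.
; Up and down moves share MovePaddle, which shifts relative Y and clamps it by mesh extent against that direction's bound.
; Size functions step the mesh's Y scale by SizeModifier within limits, or reset it.
; AddPoints and SubtractPoints both forward Count unchanged to BP_PongGameState's ScorePoint for this PlayerIndex, without counting a next round.
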(fn ConstructionScript)

(fn MovePaddle
  (params (Delta :type Float%20%28single-precision%29) (TopBounds :type Vector) (BottomBounds :type Vector))
  (bind _rootcomponent (Variables|Transformation|GetRootComponent))
  (bind _relativelocation (Variables|/Script/Engine.SceneComponent|GetRelativeLocation _rootcomponent))
  (bind _outresult (CallFunction|ClampPaddleLocation (Math|Vector|MakeVector (.x _relativelocation) (+ Delta (.y _relativelocation)) (.z _relativelocation)) TopBounds BottomBounds))
  (Transformation|SetActorRelativeLocation _outresult))

(fn ClampPaddleLocation
  (params (CurrentLocation :type Vector) (TopBounds :type Vector) (BottomBounds :type Vector))
  (bind _paddlemesh (Variables|Default|GetPaddleMesh))
  (bind _boxextent (Collision|GetComponentBounds _paddlemesh))
  (return (Math|Vector|MakeVector (.x CurrentLocation) (Math|Float|Clamp(Float) (.y CurrentLocation) (+ (.y TopBounds) (/ (.y _boxextent) 1.0)) (- (.y BottomBounds) (/ (.y _boxextent) 1.0))) (.z CurrentLocation))))

(fn MovePaddleUp
  (params (MovementSpeed :type Float%20%28single-precision%29) (AxisValue :type Float%20%28single-precision%29) (TopBounds :type Vector))
  (CallFunction|MovePaddle (* MovementSpeed AxisValue -1.0) TopBounds "0.000000,1000000000.000000, 0"))

(fn MovePaddleDown
  (params (MovementSpeed :type Float%20%28single-precision%29) (AxisValue :type Float%20%28single-precision%29) (BottomBounds :type Vector))
  (CallFunction|MovePaddle (* MovementSpeed AxisValue) "0.000000,-1000000000.000000, 0" BottomBounds))

(fn IncreasePaddleSize
  (bind _paddlemesh (Variables|Default|GetPaddleMesh))
  (bind _relativescale3d (Variables|/Script/Engine.SceneComponent|GetRelativeScale3D _paddlemesh))
  (Transformation|SetRelativeScale3D _paddlemesh (Math|Vector|MakeVector (.x _relativescale3d) (Math|Float|Clamp(Float) (+ (.y _relativescale3d) (Variables|Default|GetSizeModifier)) 0.2) (.z _relativescale3d))))

(fn ResetPaddleSize
  (Transformation|SetRelativeScale3D (Variables|Default|GetPaddleMesh) (Math|Vector|MakeVector 0.1 0.5 0.1)))

(fn DecreasePaddleSize
  (bind _paddlemesh (Variables|Default|GetPaddleMesh))
  (bind _relativescale3d (Variables|/Script/Engine.SceneComponent|GetRelativeScale3D _paddlemesh))
  (Transformation|SetRelativeScale3D _paddlemesh (Math|Vector|MakeVector (.x _relativescale3d) (Math|Float|Clamp(Float) (- (.y _relativescale3d) (Variables|Default|GetSizeModifier)) 0.2) (.z _relativescale3d))))

(fn AddPoints
  (params (Count :type Integer))
  (bind _asbp_pong_game_state (Utilities|Casting|CastToBP_PongGameState (Game|GetGameState)))
  (Default|ScorePoint _asbp_pong_game_state (Variables|Default|GetPlayerIndex) false Count))

(fn SubtractPoints
  (params (Count :type Integer))
  (bind _asbp_pong_game_state (Utilities|Casting|CastToBP_PongGameState (Game|GetGameState)))
  (Default|ScorePoint _asbp_pong_game_state (Variables|Default|GetPlayerIndex) false Count))